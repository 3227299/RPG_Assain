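; Player stats component for BP_ThirdPersonCharacter that tracks health, stamina, XP and level and writes each change straight to the character's HUD widget.
; BeginPlay waits a tick, caches the owning character and fills the HUD.
; Decrease functions return whether health or stamina is depleted, while increases clamp to the maximum.
; Reaching max XP triggers a level-up that raises the XP threshold, discards overflow XP and plays two sounds.
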(event `self.ReceiveBeginPlay`
  (bind _hud_widget (`/Game/ThirdPerson/Blueprints/BP_ThirdPersonCharacter.HUD WIDGET` (`self.PlayerCharacterBP`)))
  (`KismetSystemLibrary.DelayUntilNextTick`)
  (bind _asbp_third_person_character (cast `/Game/ThirdPerson/Blueprints/BP_ThirdPersonCharacter` (`self.GetOwner`)))
  (set `self.PlayerCharacterBP` _asbp_third_person_character)
  (`ProgressBar.SetPercent` (`/Game/UI/WB_HUD.Stamina` (`/Game/ThirdPerson/Blueprints/BP_ThirdPersonCharacter.HUD WIDGET` (`self.PlayerCharacterBP`))) (/ (`self.Current Stamina`) (`self.Max Stamina`)))
  (`ProgressBar.SetPercent` (`/Game/UI/WB_HUD.Health` _hud_widget) (/ (`self.Current Health`) (`self.MaxHealth`)))
  (`TextBlock.SetText` (`/Game/UI/WB_HUD.HealthText` _hud_widget) (`KismetTextLibrary.Conv_DoubleToText` (`self.Current Health`) "HalfToEven"))
  (`ProgressBar.SetPercent` (`/Game/UI/WB_HUD.XPBar` (`/Game/ThirdPerson/Blueprints/BP_ThirdPersonCharacter.HUD WIDGET` (`self.PlayerCharacterBP`))) (/ (`self.XP`) (`self.Max XP`)))
  (`TextBlock.SetText` (`/Game/UI/WB_HUD.XPText` (`/Game/ThirdPerson/Blueprints/BP_ThirdPersonCharacter.HUD WIDGET` (`self.PlayerCharacterBP`))) (`|FormatText` "{Current XP} / {Max XP}" (`self.XP`) (`self.Max XP`)))
  (`TextBlock.SetText` (`/Game/UI/WB_HUD.LevelText` (`/Game/ThirdPerson/Blueprints/BP_ThirdPersonCharacter.HUD WIDGET` (`self.PlayerCharacterBP`))) (`KismetTextLibrary.Conv_IntToText` (`self.Level`))))

(fn `Decrease Stamina`
  (params (`Stamina Depleted` :type "Float (double-precision)"))
  (returns (`No Stamina Left` :type Boolean))
  (if (not (<= (`self.Current Stamina`) 0.0))
    (set `self.Current Stamina` (- (`self.Current Stamina`) `Stamina Depleted`))
    (`ProgressBar.SetPercent` (`/Game/UI/WB_HUD.Stamina` (`/Game/ThirdPerson/Blueprints/BP_ThirdPersonCharacter.HUD WIDGET` (`self.PlayerCharacterBP`))) (/ (`self.Current Stamina`) (`self.Max Stamina`)))
    (if (<= (`self.Current Stamina`) 0.0)
      _
      (else
        (return false))))
  (return true))

(fn `Decreased Health`
  (params (Damage :type "Float (double-precision)"))
  (returns (`IsPlayerDead?` :type Boolean))
  (bind _hud_widget (`/Game/ThirdPerson/Blueprints/BP_ThirdPersonCharacter.HUD WIDGET` (`self.PlayerCharacterBP`)))
  (if (not (<= (`self.Current Health`) 0.0))
    (bind _output_get (set `self.Current Health` (- (`self.Current Health`) Damage)))
    (`ProgressBar.SetPercent` (`/Game/UI/WB_HUD.Health` _hud_widget) (/ _output_get (`self.MaxHealth`)))
    (`TextBlock.SetText` (`/Game/UI/WB_HUD.HealthText` _hud_widget) (`KismetTextLibrary.Conv_DoubleToText` (`self.Current Health`) "HalfToEven"))
    (if (<= (`self.Current Health`) 0.0)
      _
      (else
        (return false))))
  (return true))

(fn `Increase Health`
  (params (`Added Health` :type "Float (double-precision)"))
  (bind _hud_widget (`/Game/ThirdPerson/Blueprints/BP_ThirdPersonCharacter.HUD WIDGET` (`self.PlayerCharacterBP`)))
  (set `self.Current Health` (+ (`self.Current Health`) `Added Health`))
  (if (> (`self.Current Health`) (`self.MaxHealth`))
    (set `self.Current Health` (`self.MaxHealth`)))
  (`ProgressBar.SetPercent` (`/Game/UI/WB_HUD.Health` _hud_widget) (/ (`self.Current Health`) (`self.MaxHealth`)))
  (`TextBlock.SetText` (`/Game/UI/WB_HUD.HealthText` _hud_widget) (`KismetTextLibrary.Conv_DoubleToText` (`self.Current Health`) "HalfToEven")))

(fn `Increase Level`
  (params (`Added Level` :type Integer))
  (set `self.Level` (+ (`self.Level`) `Added Level`))
  (set `self.Max XP` (+ (`self.Max XP`) 150.0))
  (set `self.XP` 0.0)
  (`TextBlock.SetText` (`/Game/UI/WB_HUD.LevelText` (`/Game/ThirdPerson/Blueprints/BP_ThirdPersonCharacter.HUD WIDGET` (`self.PlayerCharacterBP`))) (`KismetTextLibrary.Conv_IntToText` (`self.Level`)))
  (`GameplayStatics.PlaySound2D` "/Game/Audio/UI/LevelUp1.LevelUp1" 1.0 1.0 0.0 null null)
  (`GameplayStatics.PlaySound2D` "/Game/Audio/UI/LevelUp2.LevelUp2" 1.0 1.0 0.0 null null))

(fn `Increase Max Heatlh`
  (params (Incremention :type "Float (double-precision)"))
  (bind _hud_widget (`/Game/ThirdPerson/Blueprints/BP_ThirdPersonCharacter.HUD WIDGET` (`self.PlayerCharacterBP`)))
  (set `self.MaxHealth` (+ (`self.MaxHealth`) Incremention))
  (`ProgressBar.SetPercent` (`/Game/UI/WB_HUD.Health` _hud_widget) (/ (`self.Current Health`) (`self.MaxHealth`)))
  (`TextBlock.SetText` (`/Game/UI/WB_HUD.HealthText` _hud_widget) (`KismetTextLibrary.Conv_DoubleToText` (`self.Current Health`) "HalfToEven")))

(fn `Increase Max Stamina`
  (params (`Added Stamina` :type "Float (double-precision)"))
  (set `self.Max Stamina` (+ (`self.Max Stamina`) `Added Stamina`))
  (`ProgressBar.SetPercent` (`/Game/UI/WB_HUD.Stamina` (`/Game/ThirdPerson/Blueprints/BP_ThirdPersonCharacter.HUD WIDGET` (`self.PlayerCharacterBP`))) (/ (`self.Current Stamina`) (`self.Max Stamina`))))

(fn `Increase Stamina`
  (params (`Added Stamina` :type "Float (double-precision)"))
  (set `self.Current Stamina` (+ (`self.Current Stamina`) `Added Stamina`))
  (if (> (`self.Current Stamina`) (`self.Max Stamina`))
    (set `self.Current Stamina` (`self.Max Stamina`)))
  (`ProgressBar.SetPercent` (`/Game/UI/WB_HUD.Stamina` (`/Game/ThirdPerson/Blueprints/BP_ThirdPersonCharacter.HUD WIDGET` (`self.PlayerCharacterBP`))) (/ (`self.Current Stamina`) (`self.Max Stamina`))))

(fn `Increase XP`
  (params (`Added XP` :type "Float (double-precision)"))
  (set `self.XP` (+ (`self.XP`) `Added XP`))
  (if (>= (`self.XP`) (`self.Max XP`))
    (`self.Increase Level` 1))
  (`ProgressBar.SetPercent` (`/Game/UI/WB_HUD.XPBar` (`/Game/ThirdPerson/Blueprints/BP_ThirdPersonCharacter.HUD WIDGET` (`self.PlayerCharacterBP`))) (/ (`self.XP`) (`self.Max XP`)))
  (`TextBlock.SetText` (`/Game/UI/WB_HUD.XPText` (`/Game/ThirdPerson/Blueprints/BP_ThirdPersonCharacter.HUD WIDGET` (`self.PlayerCharacterBP`))) (`|FormatText` "{Current XP} / {Max XP}" (`self.XP`) (`self.Max XP`))))