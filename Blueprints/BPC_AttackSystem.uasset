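; Melee attack component for BP_ThirdPersonCharacter that runs a four-step sword and kick combo from IA_Attack.
; Presses during an attack are buffered, and SwordAttackCombo either plays the next montage by AttackIndex or resets the combo.
; A looping timer sphere-traces between the sword points, applying rate-limited damage, camera shake and sound on "Damagable" actors.
; A separate SphereTrace event does a single-point hit check without that limit; StopSwordTrace clears the timer.
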(event `self.ReceiveBeginPlay`
  (bind _asbp_third_person_character (cast `/Game/ThirdPerson/Blueprints/BP_ThirdPersonCharacter` (`self.GetOwner`)))
  (set `self.Character BP` _asbp_third_person_character)
  (set `self.Character Mesh` (`Character.Mesh` _asbp_third_person_character)))

(event `EnhancedInput|/Game/ThirdPerson/Input/Actions/IA_Attack`
  (params (ActionValue :type Boolean) (ElapsedSeconds :type "Float (double-precision)") (TriggeredSeconds :type "Float (double-precision)") (InputAction :type "InputAction Object Reference" :default "/Game/ThirdPerson/Input/Actions/IA_Attack.IA_Attack"))
  ;[1 1 1] Attack Input
  (:`Started`
    (if (`self.can Attack?`)
      (`self.Sword Attack`)
      (`self.Start Sword Trace`))))

(event `Attack 1`
  (`/Engine/EditorBlueprintResources/StandardMacros.DoOnce` false :!label _label
    (:`Completed`
      (`KismetSystemLibrary.Delay` 0.1)
      (`|PlayMontage` (`self.Character Mesh`) "/Game/Characters/RPG_Character/Animations/SwordAttack/Attack1_Montage.Attack1_Montage"
        (:`then`
          (set `self.attack index` 1)
          (goto _label :!via `Reset`))))))

(event `Sword Attack`
  (if (`self.is Attacking?`)
    (set `self.save Attack?` true)
    (else
      (set `self.is Attacking?` true)
      (switch `int` (`self.attack index`) :!label _label_2
        (:`0`
          (`self.Attack 1`))
        (:`1`
          (`self.Attack 2`))
        (:`2`
          (`self.Attack 3`))
        (:`3`
          (`self.Attack 4`))))))

(event `Attack 2`
  (`/Engine/EditorBlueprintResources/StandardMacros.DoOnce` false :!label _label_3
    (:`Completed`
      (`KismetSystemLibrary.Delay` 0.1)
      (`|PlayMontage` (`self.Character Mesh`) "/Game/Characters/RPG_Character/Animations/SwordAttack/Attack2_Montage.Attack2_Montage"
        (:`then`
          (set `self.attack index` 2)
          (goto _label_3 :!via `Reset`))))))

(event `Sword Attack Combo`
  (if (`self.save Attack?`)
    (set `self.save Attack?` false)
    (goto _label_2)
    (else
      (`self.Stop Combo`))))

(event `Stop Combo`
  (set `self.is Attacking?` false)
  (set `self.attack index` 0))

(event `Attack 3`
  (`/Engine/EditorBlueprintResources/StandardMacros.DoOnce` false :!label _label_4
    (:`Completed`
      (`KismetSystemLibrary.Delay` 0.1)
      (`|PlayMontage` (`self.Character Mesh`) "/Game/Characters/RPG_Character/Animations/SwordAttack/Kick_Montage.Kick_Montage"
        (:`then`
          (set `self.attack index` 3)
          (goto _label_4 :!via `Reset`))))))

(event `Attack 4`
  (`/Engine/EditorBlueprintResources/StandardMacros.DoOnce` false :!label _label_5
    (:`Completed`
      (`KismetSystemLibrary.Delay` 0.1)
      (`|PlayMontage` (`self.Character Mesh`) "/Game/Characters/RPG_Character/Animations/SwordAttack/Attack3_Montage.Attack3_Montage"
        (:`then`
          (set `self.attack index` 4)
          (goto _label_5 :!via `Reset`))))))

(event `Start Sword Trace`
  (bind _returnvalue (`KismetSystemLibrary.K2_SetTimerDelegate` (delegate `Sword Trace Loop`) 0.001 true))
  (set `self.Sword TraceLoop` _returnvalue))

(event `Sword Trace Loop`
  (bind (_outhit _returnvalue) (`KismetSystemLibrary.SphereTraceSingle` :`Start` (`SceneComponent.K2_GetComponentLocation` (`/Game/ThirdPerson/Blueprints/BP_ThirdPersonCharacter.Sword Top Point` (`self.Character BP`))) :`End` (`SceneComponent.K2_GetComponentLocation` (`/Game/ThirdPerson/Blueprints/BP_ThirdPersonCharacter.Sword Bottom Point` (`self.Character BP`))) :`Radius` 12.0 :`TraceChannel` "TraceTypeQuery1" :`DrawDebugType` "ForDuration" :`DrawTime` 0.2))
  (if _returnvalue
    (bind (_bblockinghit _binitialoverlap _time _distance _location _impactpoint _normal _impactnormal _physmat _hitactor) (`GameplayStatics.BreakHitResult` _outhit))
    (if (`Actor.ActorHasTag` _hitactor "Damagable")
      (`/Engine/EditorBlueprintResources/StandardMacros.DoOnce` false :!label _label_6
        (:`Completed`
          (`GameplayStatics.ApplyDamage` _hitactor 10.0)
          (`GameplayStatics.PlayWorldCameraShake` "/Game/Blueprints/BP_HitCameraShake.BP_HitCameraShake_C" _location 0.0 2000.0)
          (`self.Play Sword Hit Sound`)
          (`KismetSystemLibrary.Delay` 0.5)
          (goto _label_6 :!via `Reset`))))))

(event `Sphere Trace`
  (bind _returnvalue (`SceneComponent.K2_GetComponentLocation` (`/Game/ThirdPerson/Blueprints/BP_ThirdPersonCharacter.Sphere Trace` (`self.Character BP`))))
  (bind (_outhit _returnvalue_2) (`KismetSystemLibrary.SphereTraceSingle` :`Start` _returnvalue :`End` _returnvalue :`Radius` 25.0 :`TraceChannel` "TraceTypeQuery1" :`DrawDebugType` "ForDuration"))
  (if _returnvalue_2
    (bind (_bblockinghit _binitialoverlap _time _distance _location _impactpoint _normal _impactnormal _physmat _hitactor) (`GameplayStatics.BreakHitResult` _outhit))
    (if (`Actor.ActorHasTag` _hitactor "Damagable")
      (if true
        (`GameplayStatics.ApplyDamage` _hitactor 10.0)
        (`GameplayStatics.PlayWorldCameraShake` "/Game/Blueprints/BP_HitCameraShake.BP_HitCameraShake_C" _location 0.0 2000.0)
        (`self.Play Sword Hit Sound`)))))

(event `Stop Sword Trace`
  (`KismetSystemLibrary.K2_ClearAndInvalidateTimerHandle` (`self.Sword TraceLoop`)))

(event `Play Sword Hit Sound`
  (`GameplayStatics.PlaySoundAtLocation` "/Game/Audio/Sword_Hits/MS_SwordHit.MS_SwordHit" (`Actor.K2_GetActorLocation` (`self.GetOwner`)) (struct) 1.0 1.0 0.0 "/Game/Audio/SA_Character.SA_Character" null null null))